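; BP_Door_1 is an interactable, lockable sliding door.
; Interact on a locked door asks the first-person player controller to use a key, then unlocks or plays a fail sound.
; An opening or closing sound plays and the IsSwinging flag is set, which Tick consumes through a FlipFlop to play or reverse a timeline.
; The timeline slides the mesh from its starting position along world X or Y, chosen by UseX.
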(event EventBeginPlay
  (Variables|Default|SetWorldStartLocation (Transformation|GetWorldLocation (Variables|Default|GetSM_Door_4))))

(event Collision|EventActorBeginOverlap
  (params (OtherActor :type Actor%20Object%20Reference)))

(event EventTick
  (params (DeltaSeconds :type Float%20%28single-precision%29))
  (bind _worldstartlocation (Variables|Default|GetWorldStartLocation))
  (bind _worldstartlocation_2 (Variables|Default|GetWorldStartLocation))
  (if (Variables|Default|GetIsSwinging)
    (Variables|Default|SetIsSwinging false)
    (Utilities|FlowControl|FlipFlop
      (:A
        (bind _doormove (Timeline|Timeline Play)
          (:Update
            (if (Variables|Default|GetUseX)
              (Transformation|SetWorldLocation (Variables|Default|GetSM_Door_4) (Math|Vector|MakeVector (+ (.x _worldstartlocation_2) (Math|Float|Lerp 0.0 1.2e+02 _doormove)) (.y _worldstartlocation_2) (.z _worldstartlocation_2)) false false)
              (else
                (Transformation|SetWorldLocation (Variables|Default|GetSM_Door_4) (Math|Vector|MakeVector (.x _worldstartlocation) (+ (.y _worldstartlocation) (Math|Float|Lerp 0.0 1.2e+02 _doormove)) (.z _worldstartlocation)) false false))))))
      (:B
        (Timeline|Timeline Reverse)))))

(event EventInteract
  (bind _sm_door_4 (Variables|Default|GetSM_Door_4))
  (bind _returnvalue (Transformation|GetWorldLocation _sm_door_4))
  (if (Variables|Default|GetIsLocked)
    (bind _asbp_first_person_player_controller (Utilities|Casting|CastToBP_FirstPersonPlayerController (Game|GetPlayerController 0)))
    (bind _keyused (Default|UseKey _asbp_first_person_player_controller))
    (if _keyused
      (Audio|PlaySoundatLocation "/Game/Audio/Ambient/DoorUnlock.DoorUnlock" _returnvalue "0, 0, 0" 1.0 1.0 0.0 0 0 0 0)
      (Variables|Default|SetIsLocked false)
      (if (not (Variables|Default|GetIsSwinging)) :!label _label
        (Variables|Default|SetIsSwinging true)
        (if (Variables|Default|GetIsOpen)
          (Audio|PlaySoundatLocation "/Game/Audio/Ambient/DoorClose.DoorClose" _returnvalue "0, 0, 0" 2.0 1.0 0.0 0 0 0 0)
          (else
            (Audio|PlaySoundatLocation "/Game/Audio/Ambient/DoorOpen.DoorOpen" _returnvalue "0, 0, 0" 2.0 1.0 0.0 0 0 0 0))))
      (else
        (Audio|PlaySoundatLocation "/Game/Audio/Ambient/DoorFail.DoorFail" _returnvalue "0, 0, 0" 1.0 1.0 0.0 0 0 0 0)))
    (else
      (Development|PrintString "Hello")
      (goto _label))))

(fn ConstructionScript)