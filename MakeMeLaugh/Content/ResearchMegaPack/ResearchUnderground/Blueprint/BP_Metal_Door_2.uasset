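; Metal door that either slides open or, when flagged as the end door, serves as the game's exit.
; BeginPlay records the starting height of the Left component and sets decal visibility from a flag.
; Open raises Left vertically along a timeline, only once, with no close logic.
; On an end door, Open instead shows the Escaped widget and switches the player to UI-only input with a visible cursor.
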(event Custom|Open
  (bind _returnvalue (Game|GetPlayerController 0))
  (bind _left (Variables|Default|GetLeft))
  (bind _returnvalue_2 (Transformation|GetWorldLocation _left))
  (if (not (Variables|Default|GetIsOpen))
    (if (Variables|Default|GetIsEndDoor)
      (bind _returnvalue_3 (UserInterface|CreateWidget "/Game/UI/Escaped.Escaped_C"))
      (UserInterface|Viewport|AddtoViewport _returnvalue_3 0)
      (Input|SetInputModeUIOnly _returnvalue _returnvalue_3 "DoNotLock" false)
      (Variables|/Script/Engine.PlayerController|SetbShowMouseCursor _returnvalue true)
      (else
        (Variables|Default|SetIsOpen true)
        (bind _newtrack_0 (Timeline|Timeline Play)
          (:Update
            (Transformation|SetWorldLocation _left (Math|Vector|MakeVector (.x _returnvalue_2) (.y _returnvalue_2) (+ (Variables|Default|GetStartWorldZ) (Math|Float|Lerp 0.0 3e+02 _newtrack_0))) false false)))))))

(event EventBeginPlay
  (Variables|Default|SetStartWorldZ (.z (Transformation|GetWorldLocation (Variables|Default|GetLeft))))
  (Development|SetHiddeninGame (Variables|Default|GetDecal) (Variables|Default|GetHideDecal) false))

(fn ConstructionScript)