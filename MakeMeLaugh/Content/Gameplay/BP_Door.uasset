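; BP_Door is an interactable door that swings its mesh around the yaw axis.
; Interact prints a debug string, then starts the swing and stores the starting yaw if it is not already swinging.
; Tick rotates the mesh at a fixed angle per TimeToSwing, with direction set by IsOpen.
; The graph is unfinished: it never clears IsSwinging, toggles IsOpen or reads the stored yaw, so the swing never stops.
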(event EventBeginPlay)

(event Collision|EventActorBeginOverlap
  (params (OtherActor :type Actor%20Object%20Reference)))

(event EventTick
  (params (DeltaSeconds :type Float%20%28single-precision%29))
  (bind _timetoswing (Variables|Default|GetTimeToSwing))
  (bind _returnvalue (/ DeltaSeconds _timetoswing))
  (bind _returnvalue_2 (* _returnvalue 7e+01))
  (if (Variables|Default|GetIsSwinging)
    (if (Variables|Default|GetIsOpen)
      (Transformation|AddWorldRotation (Variables|Default|GetDoorMesh) (Math|Rotator|MakeRotator 0.0 0.0 _returnvalue_2) false false)
      (else
        (Transformation|AddWorldRotation (Variables|Default|GetDoorMesh) (Math|Rotator|MakeRotator 0.0 0.0 (* _returnvalue_2 -1.0)) false false)))))

(event EventInteract
  (Development|PrintString "Hello")
  (if (not (Variables|Default|GetIsSwinging))
    (Variables|Default|SetIsSwinging true)
    (Variables|Default|SetSwingStartRotation (.yaw (Transformation|GetWorldRotation (Variables|Default|GetDoorMesh))))))

(fn ConstructionScript)