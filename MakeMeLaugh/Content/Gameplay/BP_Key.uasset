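; BP_Key is an interactable key pickup for a first-person game.
; On Interact it calls GiveKey on BP_FirstPersonPlayerController, plays a paper sound at the key's location and destroys itself.
; Every Tick it reads that controller's BabyLaughMeter and shows its Widget component only while the meter is at least 0.8, hiding it otherwise.
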(event EventBeginPlay)

(event Collision|EventActorBeginOverlap
  (params (OtherActor :type Actor%20Object%20Reference)))

(event EventInteract
  (bind _asbp_first_person_player_controller (Utilities|Casting|CastToBP_FirstPersonPlayerController (Game|GetPlayerController 0)))
  (Default|GiveKey _asbp_first_person_player_controller)
  (Audio|PlaySoundatLocation "/Game/Audio/ItemNoise/Misc_Paper_01.Misc_Paper_01" (Transformation|GetWorldLocation (Variables|Default|GetKey)) "0, 0, 0" 1.0 1.0 0.0 0 0 0 0)
  (Actor|DestroyActor))

(event EventTick
  (params (DeltaSeconds :type Float%20%28single-precision%29))
  (bind _asbp_first_person_player_controller (Utilities|Casting|CastToBP_FirstPersonPlayerController (Game|GetPlayerController 0)))
  (Development|SetHiddeninGame (Variables|Default|GetWidget) (not (>= (Variables|/Game/FirstPerson/Blueprints/BP_FirstPersonPlayerController.BP_FirstPersonPlayerController_C|GetBabyLaughMeter _asbp_first_person_player_controller) 0.8)) false))

(fn ConstructionScript)