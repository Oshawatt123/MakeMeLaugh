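; BP_BigBadCharacter is an AI enemy character that detects the player and feeds CanSeePlayer, CanHearPlayer and SearchLocation to its Blackboard.
; Tick checks sight with an unnormalized forward dot product, distance limit and visibility trace instead of PawnSensing, whose event does nothing.
; NoiseHeard records the player's location and starts a hearing timer, which Tick counts down.
; SetWalk and SetRun switch movement speed.
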(event OnSeePawn(PawnSensing)
  (params (Pawn :type Pawn%20Object%20Reference)))

(event EventBeginPlay)

(event Collision|EventActorBeginOverlap
  (params (OtherActor :type Actor%20Object%20Reference)))

(event EventTick
  (params (DeltaSeconds :type Float%20%28single-precision%29))
  (bind _returnvalue (Game|GetPlayerCharacter 0))
  (bind _self self)
  (bind _capsulecomponent (Variables|Collision|GetCapsuleComponent))
  (bind _returnvalue_2 (Transformation|GetActorLocation _returnvalue))
  (bind _returnvalue_3 (Transformation|GetWorldLocation _capsulecomponent))
  (bind _returnvalue_4 (AI|GetAIController _self))
  (bind _returnvalue_5 (AI|GetBlackboard _returnvalue_4))
  (bind _returnvalue_6 (- _returnvalue_2 _returnvalue_3))
  (bind _output_get (Variables|Default|SetHearTimer (- (Variables|Default|GetHearTimer) DeltaSeconds)))
  (AI|Components|Blackboard|SetValueasBool (AI|GetBlackboard (AI|GetAIController self)) (Utilities|Name|MakeLiteralName "CanHearPlayer") (> _output_get 0.0))
  (if (> (Math|Vector|DotProduct (Math|Vector|GetForwardVector _capsulecomponent) _returnvalue_6) 0.2)
    (if (< (Math|Vector|VectorLength _returnvalue_6) (Variables|Default|GetSeeDistance))
      (bind (_outhit _returnvalue_7) (Collision|LineTraceByChannel _returnvalue_3 (+ _returnvalue_2 (* _returnvalue_6 5e+01)) "TraceTypeQuery1" false 0 "ForOneFrame"))
      (if _returnvalue_7
        (bind _asbp_first_person_character (Utilities|Casting|CastToBP_FirstPersonCharacter (.HitActor (Collision|BreakHitResult _outhit)))
          (:then
            (AI|Components|Blackboard|SetValueasBool _returnvalue_5 (Utilities|Name|MakeLiteralName "CanSeePlayer") true)
            (AI|Components|Blackboard|SetValueasVector _returnvalue_5 (Utilities|Name|MakeLiteralName "SearchLocation") (Transformation|GetActorLocation _asbp_first_person_character)))
          (:CastFailed
            (AI|Components|Blackboard|SetValueasBool _returnvalue_5 (Utilities|Name|MakeLiteralName "CanSeePlayer") false :!label _label)))
        (else
          (goto _label)))
      (else
        (goto _label)))
    (else
      (goto _label))))

(fn ConstructionScript)

(fn NoiseHeard
  (params (SoundTime :type Float%20%28double-precision%29))
  (bind _self self)
  (bind _returnvalue (AI|GetAIController _self))
  (bind _returnvalue_2 (AI|GetBlackboard _returnvalue))
  (Variables|Default|SetHearTimer SoundTime)
  (Development|PrintString "NoiseHeard")
  (AI|Components|Blackboard|SetValueasBool _returnvalue_2 (Utilities|Name|MakeLiteralName "CanHearPlayer") true)
  (AI|Components|Blackboard|SetValueasVector _returnvalue_2 (Utilities|Name|MakeLiteralName "SearchLocation") (Transformation|GetActorLocation (Game|GetPlayerCharacter 0))))

(fn SetWalk
  (Variables|/Script/Engine.CharacterMovementComponent|SetMaxWalkSpeed (Variables|Character|GetCharacterMovement) 2e+02))

(fn SetRun
  (Variables|/Script/Engine.CharacterMovementComponent|SetMaxWalkSpeed (Variables|Character|GetCharacterMovement) 4.5e+02))